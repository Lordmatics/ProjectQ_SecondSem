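; Player character Blueprint that drives full-screen post-process feedback for acid bile and damage.
; BeginPlay creates dynamic instances of the acid and damage materials and adds them to the PostProcessComponent as blendables.
; Each Tick, the InBile and GotHit flags play or reverse two timelines, fading the acid's EffectStrength and shrinking the damage MaskRadius.
; C and V keys also trigger the bile and damage effects directly.
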(event Custom|ScreenBile
  (bind _newtrack_0 (Timeline|Timeline_0 Play)
    (:Update
      (Rendering|Material|SetScalarParameterValue (Variables|Default|GetM_Bile) "EffectStrength" (Math|Float|Lerp 0.0 1.0 _newtrack_0) :!class /Script/Engine.MaterialInstanceDynamic))))

(event Custom|ScreenBileOff
  (bind _newtrack_0 (Timeline|Timeline_0 Reverse)
    (:Update
      (Rendering|Material|SetScalarParameterValue (Variables|Default|GetM_Bile) "EffectStrength" (Math|Float|Lerp 0.0 1.0 _newtrack_0) :!class /Script/Engine.MaterialInstanceDynamic))))

(event Custom|ScreenDamage
  (bind _newtrack_1 (Timeline|Timeline_1 Play)
    (:Update
      (Rendering|Material|SetScalarParameterValue (Variables|Default|GetM_Blood) "MaskRadius" (Math|Float|Lerp 2.0 0.0 _newtrack_1) :!class /Script/Engine.MaterialInstanceDynamic))))

(event Custom|ScreenDamageOff
  (bind _newtrack_1 (Timeline|Timeline_1 Reverse)
    (:Update
      (Rendering|Material|SetScalarParameterValue (Variables|Default|GetM_Blood) "MaskRadius" (Math|Float|Lerp 2.0 0.0 _newtrack_1) :!class /Script/Engine.MaterialInstanceDynamic))))

(event EventBeginPlay
  (bind _postprocesscomponent (Variables|Default|GetPostProcessComponent))
  (bind _returnvalue (Rendering|Material|CreateDynamicMaterialInstance "/Game/PostProcess/MPP_Acid.MPP_Acid" :!class /Script/Engine.KismetMaterialLibrary))
  (bind _output_get (Variables|Default|SetM_Bile _returnvalue))
  (Rendering|AddorUpdateBlendable _postprocesscomponent _output_get 1.0 :!class /Script/Engine.PostProcessComponent)
  (bind _returnvalue_2 (Rendering|Material|CreateDynamicMaterialInstance "/Game/PostProcess/MPP_Damage.MPP_Damage" :!class /Script/Engine.KismetMaterialLibrary))
  (bind _output_get_2 (Variables|Default|SetM_Blood _returnvalue_2))
  (Rendering|AddorUpdateBlendable _postprocesscomponent _output_get_2 1.0 :!class /Script/Engine.PostProcessComponent))

(event EventTick
  (params (DeltaSeconds :type Float%20%28single-precision%29))
  (Utilities|FlowControl|Sequence
    (:then_0
      (if (Variables|Default|GetbInBile)
        (CallFunction|ScreenBile)
        (else
          (CallFunction|ScreenBileOff))))
    (:then_1
      (if (Variables|Default|GetbGotHit)
        (CallFunction|ScreenDamage)
        (else
          (CallFunction|ScreenDamageOff))))))

(event Input|KeyboardEvents|C
  (params (Key :type Key%20Structure :default "AnyKey"))
  (:Pressed
    (CallFunction|ScreenBile)))

(event Input|KeyboardEvents|V
  (params (Key :type Key%20Structure :default "AnyKey"))
  (:Pressed
    (CallFunction|ScreenDamage)))

(fn ConstructionScript)